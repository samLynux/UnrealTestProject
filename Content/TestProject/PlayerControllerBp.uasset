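; Player controller Blueprint that sets up the main HUD and a manual save hotkey.
; When play begins for a local controller, it creates the Main_HUD widget, adds it to the viewport and switches input to game only.
; Pressing L casts the game mode to SGameModeBase, writes the save game and prints a confirmation.
; The pawn-change handler is empty and its binding is never executed.
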(event `OnPawnChanged_Event` :!signature `self.OnPawnChanged`
  (params (NewPawn :type "Pawn Object Reference")))

(event `self.ReceiveBeginPlay`)

(event `self.BlueprintBeginPlayingState`
  (if (`self.IsLocalController`)
    (bind _returnvalue (`|CreateWidget` "/Game/TestProject/UI/Main_HUD.Main_HUD_C"))
    (`UserWidget.AddToViewport` _returnvalue 0)
    (`WidgetBlueprintLibrary.SetInputMode_GameOnly` self)))

(event `Key|L`
  (params (Key :type "Key Structure"))
  (:`Pressed`
    (bind _assgame_mode_base (cast `SGameModeBase` (`GameplayStatics.GetGameMode`)))
    (`SGameModeBase.WriteSaveGame` _assgame_mode_base)
    (`KismetSystemLibrary.PrintString` "save")))

(fn `UserConstructionScript`)